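; Base AI character that patrols the points of an assigned MovementSpline, starting on BeginPlay when one is set.
; FollowSpline runs AI MoveTo to the current point, then on success advances the index, wraps past the end, waits briefly and calls itself again.
; Pawn Sensing and AI Perception events only print debug messages, and ChasePlayer is an empty stub.
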(event OnSeePawn(PawnSensing)
  (params (Pawn :type Pawn%20Object%20Reference))
  (Development|PrintString (Utilities|String|Append "You're seen by" (Utilities|GetDisplayName self))))

(event OnHearNoise(PawnSensing)
  (params (Instigator :type Pawn%20Object%20Reference) (Location :type Vector%20%28by%20ref%29 :default "0, 0, 0") (Volume :type Float%20%28single-precision%29))
  (Development|PrintString "Heard something"))

(event OnTargetPerceptionUpdated(AIPerception)
  (params (Actor :type Actor%20Object%20Reference) (Stimulus :type AI%20Stimulus%20Structure))
  (if (.bSuccessfullySensed (Utilities|Struct|BreakAIStimulus Stimulus))
    (Development|PrintString "sensed")))

(event OnPerceptionUpdated(AIPerception)
  (params (UpdatedActors :type Array%20of%20Actor%20Object%20References))
  (Development|PrintString "updated"))

(event Custom|FollowSpline
  (bind _movementresult (AI|AIMoveTo self (CallFunction|Destination) 0 5.0 false)
    (:then
      (switch Utilities|FlowControl|Switch|SwitchonEPathFollowingResult _movementresult
        (:Blocked
          (Development|PrintString (Utilities|String|Append (Utilities|GetObjectName self) "somewhere")))))
    (:OnSuccess
      (bind _result (Math|Integer|IncrementInt (Variables|Default|GetCurrentWaypointIndex))
        (:%20%20
          (if (> _result (Spline|GetNumberOfSplinePoints (Variables|/Game/BluePrints/Character/IAs/BP_AIFollowedSpline.BP_AIFollowedSpline_C|GetSpline (Variables|Default|GetMovementSpline))))
            (Variables|Default|SetCurrentWaypointIndex 0))
          (Utilities|FlowControl|Delay 1.0)
          (CallFunction|FollowSpline))))))

(event Custom|ChasePlayer)

(event EventBeginPlay
  (Variables|Default|GetMovementSpline
    (:then
      (CallFunction|FollowSpline))
    (:else)))

(event Collision|EventActorBeginOverlap
  (params (OtherActor :type Actor%20Object%20Reference)))

(event EventTick
  (params (DeltaSeconds :type Float%20%28single-precision%29)))

(fn ConstructionScript
  (|CallParentFunction))

(fn Destination
  (return (.Position (Utilities|Struct|BreakSplinePoint (Spline|GetSplinePointAt (Variables|/Game/BluePrints/Character/IAs/BP_AIFollowedSpline.BP_AIFollowedSpline_C|GetSpline (Variables|Default|GetMovementSpline)) (Variables|Default|GetCurrentWaypointIndex) "World")))))