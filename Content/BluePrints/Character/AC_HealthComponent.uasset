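; Actor component that holds a character's health, with functions for taking damage and healing.
; BeginPlay sets CurrentHealth to MaxHealth, and Tick is unused.
; TakeDamage, skipped under Invincibility, stores DamageValue minus CurrentHealth (operands reversed), clamped between zero and current health.
; Heal adds HealValue but also clamps to CurrentHealth instead of MaxHealth, so it cannot raise health.
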(event EventBeginPlay
  (Variables|Default|SetCurrentHealth (Variables|Default|GetMaxHealth)))

(event EventTick
  (params (DeltaSeconds :type Float%20%28single-precision%29)))

(fn TakeDamage
  (params (DamageValue :type Integer))
  (if (not (Variables|Default|GetInvincibility))
    (Variables|Default|SetCurrentHealth (Math|Integer|Clamp(Integer) (- DamageValue (Variables|Default|GetCurrentHealth)) 0 (Variables|Default|GetCurrentHealth)))))

(fn Heal
  (params (HealValue :type Integer))
  (Variables|Default|SetCurrentHealth (Math|Integer|Clamp(Integer) (+ HealValue (Variables|Default|GetCurrentHealth)) 0 (Variables|Default|GetCurrentHealth))))