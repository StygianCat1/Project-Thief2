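; BP_Camera is a surveillance camera that sweeps back and forth and raises a noise alarm when it sees BP_Garett.
; A timeline ping-pongs its yaw around the starting rotation by DegreeRotation.
; When PawnSensing spots Garett either visible or moving, it reports noise at the ground point traced beneath the camera at BeginPlay.
; The sweep then stops and a timer resumes it in the same direction.
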(event OnSeePawn(PawnSensing)
  (params (Pawn :type Pawn%20Object%20Reference))
  (bind _asbp_garett (Utilities|Casting|CastToBP_Garett Pawn))
  (if (Variables|/Game/BluePrints/Character/Garett/BP_Garett.BP_Garett_C|GetVisible _asbp_garett)
    (Utilities|Time|ClearandInvalidateTimerbyHandle (Variables|Default|GetTimerRef) :!label _label)
    (Class|AISenseHearing|ReportNoiseEvent (Variables|Default|GetNoisePointLocation) 1.0 self 4e+03 "None")
    (CallFunction|StoponSeePlayer)
    (bind _returnvalue (Utilities|Time|SetTimerbyFunctionName 0 "PlayBack" 5.0))
    (Utilities|FlowControl|DoOnce false
      (:Completed
        (Variables|Default|SetTimerRef _returnvalue)))
    (elif (Variables|/Game/BluePrints/Character/BP_FirstPersonCharacter.BP_FirstPersonCharacter_C|GetMoving _asbp_garett)
      (goto _label))))

(event Custom|CameraMovement
  (bind _camerarotation (Variables|Default|GetCameraRotation))
  (bind (_direction _camerarotation_2) (Timeline|MovementTimeline Play)
    (:Update
      (Transformation|SetWorldRotation (Variables|Default|GetDefaultSceneRoot) (Math|Rotator|MakeRotator (.roll _camerarotation) (.pitch _camerarotation) (+ (.yaw _camerarotation) (* _camerarotation_2 (Variables|Default|GetDegreeRotation)))) false false))
    (:Finished
      (switch Utilities|FlowControl|Switch|SwitchonETimelineDirection _direction
        (:Forward
          (Timeline|MovementTimeline Reverse))
        (:Backward
          (Timeline|MovementTimeline Play))))))

(event Custom|StopOnSeePlayer
  (bind _camerarotation (Variables|Default|GetCameraRotation))
  (bind (_direction _camerarotation_2) (Timeline|MovementTimeline Stop)
    (:Update
      (Transformation|SetWorldRotation (Variables|Default|GetDefaultSceneRoot) (Math|Rotator|MakeRotator (.roll _camerarotation) (.pitch _camerarotation) (+ (.yaw _camerarotation) (* _camerarotation_2 (Variables|Default|GetDegreeRotation)))) false false))
    (:Finished
      (switch Utilities|FlowControl|Switch|SwitchonETimelineDirection _direction
        (:Forward
          (Timeline|MovementTimeline Reverse))
        (:Backward
          (Timeline|MovementTimeline Play))))))

(event Custom|PlayBack
  (bind _camerarotation (Variables|Default|GetCameraRotation))
  (switch Utilities|FlowControl|Switch|SwitchonETimelineDirection (stale _direction)
    (:Forward
      (bind (_direction _camerarotation_2) (Timeline|MovementTimeline Play)
        (:Update
          (Transformation|SetWorldRotation (Variables|Default|GetDefaultSceneRoot) (Math|Rotator|MakeRotator (.roll _camerarotation) (.pitch _camerarotation) (+ (.yaw _camerarotation) (* _camerarotation_2 (Variables|Default|GetDegreeRotation)))) false false))
        (:Finished
          (switch Utilities|FlowControl|Switch|SwitchonETimelineDirection _direction
            (:Forward
              (Timeline|MovementTimeline Reverse))
            (:Backward
              (Timeline|MovementTimeline Play))))))
    (:Backward
      (Timeline|MovementTimeline Reverse))))

(event EventBeginPlay
  (bind _returnvalue (Transformation|GetActorLocation))
  (bind (_x _y _z) (Math|Vector|BreakVector _returnvalue))
  (bind _outhit (Collision|LineTraceByChannel _returnvalue (Math|Vector|MakeVector _x _y (- _z 1e+04)) "TraceTypeQuery1" false 0 "None"))
  (Variables|Default|SetNoisePointLocation (.ImpactPoint (Collision|BreakHitResult _outhit)))
  (Variables|Default|SetCameraRotation (Transformation|GetWorldRotation (Variables|Default|GetDefaultSceneRoot)))
  (CallFunction|CameraMovement))

(fn ConstructionScript)