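; BP_ExteriorEnvironment is a trigger volume that hides chosen static mesh actors while the BP_Garett character is inside it.
; When BP_Garett begins overlapping the Box, every actor in StaticMeshActorRef is hidden and loses its collision.
; When the overlap ends, the same actors are shown again with collision restored.
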(event OnComponentBeginOverlap(Box)
  (params (OverlappedComponent :type Primitive%20Component%20Object%20Reference) (OtherActor :type Actor%20Object%20Reference) (OtherComp :type Primitive%20Component%20Object%20Reference) (OtherBodyIndex :type Integer) (bFromSweep :type Boolean) (SweepResult :type Hit%20Result%20Structure%20%28by%20ref%29))
  ;[0.15 0.15 0.15 0.5] Hide & show chosen static mesh
  (Utilities|Casting|CastToBP_Garett OtherActor)
  (for _array_element (Variables|Default|GetStaticMeshActorRef)
    (Rendering|SetActorHiddenInGame _array_element true)
    (Collision|SetActorEnableCollision _array_element false)))

(event OnComponentEndOverlap(Box)
  (params (OverlappedComponent :type Primitive%20Component%20Object%20Reference) (OtherActor :type Actor%20Object%20Reference) (OtherComp :type Primitive%20Component%20Object%20Reference) (OtherBodyIndex :type Integer))
  ;[0.15 0.15 0.15 0.5] Hide & show chosen static mesh
  (Utilities|Casting|CastToBP_Garett OtherActor)
  (for _array_element (Variables|Default|GetStaticMeshActorRef)
    (Rendering|SetActorHiddenInGame _array_element false)
    (Collision|SetActorEnableCollision _array_element true)))

(event EventBeginPlay)

(fn ConstructionScript)