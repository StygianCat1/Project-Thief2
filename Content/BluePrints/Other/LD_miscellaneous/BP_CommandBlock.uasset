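; BP_CommandBlock is a drone hack station that disables chosen cameras and hacks doors.
; On BeginPlay it binds to a Hacked event dispatcher, which fires a one-shot response through a DoOnce.
; That response turns the sphere red, then calls StopEverything on each referenced camera and Hackdoor on each referenced door.
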(event Custom|ChosenCameraStop
  ;[0.15 0.15 0.15 0.5] Drone hack station, stop chosen camera from working
  (Utilities|FlowControl|DoOnce false
    (:Completed
      (Rendering|Material|SetMaterial (Variables|Default|GetSphere) 0 "/Game/Assets/Material/MI_Red.MI_Red")
      (for _array_element (Variables|Default|GetCameraRef)
        (Default|StopEverything _array_element))
      (for _array_element_2 (Variables|Default|GetDoorsRef)
        (Default|Hackdoor _array_element_2)))))

(event EventBeginPlay
  ;[0.15 0.15 0.15 0.5] Drone hack station, stop chosen camera from working
  (EventDispatchers|BindEventtoHacked (delegate Custom|ChosenCameraStop)))

(fn ConstructionScript)