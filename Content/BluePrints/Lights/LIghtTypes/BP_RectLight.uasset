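; BP_RectLight is a light-type Blueprint with an AI Perception component that reacts when it senses the BP_Garett character.
; On each target perception update for BP_Garett, a FlipFlop alternates debug prints of "Saw" and "Hidden".
; The state is inferred from alternation alone, as the stimulus itself is not checked.
; Other events are disabled stubs, and the construction script only calls its parent.
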(event OnTargetPerceptionUpdated(AIPerception)
  (params (Actor :type Actor%20Object%20Reference) (Stimulus :type AI%20Stimulus%20Structure))
  (Utilities|Casting|CastToBP_Garett Actor)
  (Utilities|FlowControl|FlipFlop
    (:A
      (Development|PrintString "Saw"))
    (:B
      (Development|PrintString "Hidden"))))

(event EventBeginPlay
  (|CallParentFunction) ; This node is disabled and will not be called.\nDrag off pins to build functionality.
)

(event Collision|EventActorBeginOverlap
  (params (OtherActor :type Actor%20Object%20Reference))
  (|CallParentFunction OtherActor) ; This node is disabled and will not be called.\nDrag off pins to build functionality.
)

(event EventTick
  (params (DeltaSeconds :type Float%20%28single-precision%29))
  (|CallParentFunction DeltaSeconds) ; This node is disabled and will not be called.\nDrag off pins to build functionality.
)

(fn ConstructionScript
  (|CallParentFunction))