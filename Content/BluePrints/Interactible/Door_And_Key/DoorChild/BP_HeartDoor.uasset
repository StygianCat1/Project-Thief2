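; BP_HeartDoor is a door child Blueprint that requires a heart key from the interacting character.
; It overrides VerifyKey to return true when the character's Keys struct holds at least one HeartKey.
; The construction script only calls the parent, and the event nodes are disabled stubs, so all other door behavior comes from the parent class.
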(event EventBeginPlay
  (|CallParentFunction) ; This node is disabled and will not be called.\nDrag off pins to build functionality.
)

(event Collision|EventActorBeginOverlap
  (params (OtherActor :type Actor%20Object%20Reference))
  (|CallParentFunction OtherActor) ; This node is disabled and will not be called.\nDrag off pins to build functionality.
)

(event EventTick
  (params (DeltaSeconds :type Float%20%28single-precision%29))
  (|CallParentFunction DeltaSeconds) ; This node is disabled and will not be called.\nDrag off pins to build functionality.
)

(fn ConstructionScript
  (|CallParentFunction))

(fn VerifyKey
  (params (Character :type BP%20Garett%20Object%20Reference))
  ;[0.15 0.15 0.15 0.5] Key verification
  (return (>= (Variables|/Game/BluePrints/Interactible/Door_And_Key/Data/PDA_Keys.PDA_Keys_C|GetHeartKey (Variables|/Game/BluePrints/Character/BP_FirstPersonCharacter.BP_FirstPersonCharacter_C|GetKeys Character)) 1)))