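; Interactible door that swings left or right around a pivot, toggled by a key-checked interaction or by a Hackdoor event.
; Box overlap binds and unbinds the key check to BP_Garett's interact, acting only when the grabbed component belongs to this door.
; A DoOnce and FlipFlop alternate opening and closing timelines, blocking re-entry until each finishes.
; VerifyKey always returns false here, so key interaction only prints a refusal.
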(event OnComponentBeginOverlap(BoxCollision)
  (params (OverlappedComponent :type Primitive%20Component%20Object%20Reference) (OtherActor :type Actor%20Object%20Reference) (OtherComp :type Primitive%20Component%20Object%20Reference) (OtherBodyIndex :type Integer) (bFromSweep :type Boolean) (SweepResult :type Hit%20Result%20Structure%20%28by%20ref%29))
  ;[0.15 0.15 0.15 0.5] Bind event for reaction
  (bind _asbp_garett (Utilities|Casting|CastToBP_Garett OtherActor))
  (bind _output_get (Variables|Default|SetCharacterRef _asbp_garett))
  (EventDispatchers|BindEventtoInteract _output_get (delegate Custom|OpenDoorWithKey)))

(event OnComponentEndOverlap(BoxCollision)
  (params (OverlappedComponent :type Primitive%20Component%20Object%20Reference) (OtherActor :type Actor%20Object%20Reference) (OtherComp :type Primitive%20Component%20Object%20Reference) (OtherBodyIndex :type Integer))
  ;[0.15 0.15 0.15 0.5] Unbind event to not be mistaken
  (bind _asbp_garett (Utilities|Casting|CastToBP_Garett OtherActor))
  (EventDispatchers|UnbindEventfromInteract _asbp_garett (delegate Custom|OpenDoorWithKey)))

(event Custom|OpenDoorWithKey
  (bind _doorpivotpoint (Variables|Default|GetDoorPivotPoint))
  (bind _doorpivotpoint_2 (Variables|Default|GetDoorPivotPoint))
  ;[0.15 0.15 0.15 0.5] Verify interaction
  (if (== (Components|GetOwner (Variables|/Game/BluePrints/Character/Garett/BP_Garett.BP_Garett_C|GetGrabbedComponent (Variables|Default|GetCharacterRef))) self)
    ;[0.15 0.15 0.15 0.5] Verification if key owned
    (bind _canopendoor (CallFunction|VerifyKey (Variables|Default|GetCharacterRef)))
    (if _canopendoor
      ;[0.15 0.15 0.15 0.5] Door opening / closing
      (Utilities|FlowControl|DoOnce false :!label _label
        (:Completed
          (Utilities|FlowControl|FlipFlop
            (:A
              (bind _doormovement (Timeline|DoorOpening PlayFromStart)
                (:Update
                  (Transformation|SetWorldRotation _doorpivotpoint_2 (Math|Rotator|MakeRotator 0.0 0.0 (+ (* (.X (Math|Vector|BreakVector _doormovement)) (Variables|Default|GetDoorOpeningDegree)) (.Roll (Math|Rotator|BreakRotator (Transformation|GetWorldRotation _doorpivotpoint_2))))) true false))
                (:Finished
                  (goto _label Reset))))
            (:B
              (bind _doormovement_2 (Timeline|DoorClosing ReverseFromEnd)
                (:Update
                  (Transformation|SetWorldRotation _doorpivotpoint (Math|Rotator|MakeRotator 0.0 0.0 (+ (* (.X (Math|Vector|BreakVector _doormovement_2)) (Variables|Default|GetDoorOpeningDegree)) (.Roll (Math|Rotator|BreakRotator (Transformation|GetWorldRotation _doorpivotpoint))))) true false))
                (:Finished
                  (goto _label Reset)))))))
      (else
        (Development|PrintString "Can Not Open")))))

(event Custom|Hackdoor
  (bind _doorpivotpoint (Variables|Default|GetDoorPivotPoint))
  (bind _doorpivotpoint_2 (Variables|Default|GetDoorPivotPoint))
  ;[0.15 0.15 0.15 0.5] Door opening / closing
  (Utilities|FlowControl|DoOnce false :!label _label
    (:Completed
      (Utilities|FlowControl|FlipFlop
        (:A
          (bind _doormovement (Timeline|DoorOpening PlayFromStart)
            (:Update
              (Transformation|SetWorldRotation _doorpivotpoint_2 (Math|Rotator|MakeRotator 0.0 0.0 (+ (* (.X (Math|Vector|BreakVector _doormovement)) (Variables|Default|GetDoorOpeningDegree)) (.Roll (Math|Rotator|BreakRotator (Transformation|GetWorldRotation _doorpivotpoint_2))))) true false))
            (:Finished
              (goto _label Reset))))
        (:B
          (bind _doormovement_2 (Timeline|DoorClosing ReverseFromEnd)
            (:Update
              (Transformation|SetWorldRotation _doorpivotpoint (Math|Rotator|MakeRotator 0.0 0.0 (+ (* (.X (Math|Vector|BreakVector _doormovement_2)) (Variables|Default|GetDoorOpeningDegree)) (.Roll (Math|Rotator|BreakRotator (Transformation|GetWorldRotation _doorpivotpoint))))) true false))
            (:Finished
              (goto _label Reset))))))))

(event EventBeginPlay
  ;[0.15 0.15 0.15 0.5] Door rotation direction
  (switch Utilities|FlowControl|Switch|SwitchonE_DoorRotation (Variables|Default|GetRotateTo)
    (:NewEnumerator0
      (Variables|Default|SetDoorOpeningDegree (Variables|Default|GetDoorOpeningDegree)))
    (:NewEnumerator1
      (Variables|Default|SetDoorOpeningDegree (* (Variables|Default|GetDoorOpeningDegree) -1.0)))))

(fn ConstructionScript)

(fn VerifyKey
  (params (Character :type BP%20Garett%20Object%20Reference))
  (return false))