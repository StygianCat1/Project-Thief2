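; BP_PickUpCollectables is a pickable collectable that shows readable content on screen when picked up.
; Its PickUp function creates a WBP_Collectables widget, fills the title, body and signature from its own Titre, Text and Signature variables, and adds it to the viewport.
; The event graph is inactive, and PickUp itself neither removes the actor nor records the collection.
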(event EventBeginPlay)

(event Collision|EventActorBeginOverlap
  (params (OtherActor :type Actor%20Object%20Reference)))

(event EventTick
  (params (DeltaSeconds :type Float%20%28single-precision%29)))

(fn ConstructionScript
  (|CallParentFunction))

(fn PickUp
  (bind _returnvalue (UserInterface|CreateWidget "/Game/UI/WBP_Collectables.WBP_Collectables_C"))
  (Variables|/Script/UMG.TextBlock|SetText (Variables|/Game/UI/WBP_Collectables.WBP_Collectables_C|GetTitle _returnvalue) (Utilities|Text|ToText(Name) (Variables|Default|GetTitre)))
  (Variables|/Script/UMG.TextBlock|SetText (Variables|/Game/UI/WBP_Collectables.WBP_Collectables_C|GetText _returnvalue) (Variables|Default|GetText))
  (Variables|/Script/UMG.TextBlock|SetText (Variables|/Game/UI/WBP_Collectables.WBP_Collectables_C|GetSignature _returnvalue) (Variables|Default|GetSignature))
  (UserInterface|Viewport|AddtoViewport _returnvalue 0))