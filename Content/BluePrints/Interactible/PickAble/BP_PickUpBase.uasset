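; Base pickup actor that shows a configurable mesh, with physics off, and serves as a parent for interactable pickups.
; Box overlap binds and unbinds its check to the interact event of BP_Garett.
; On interact, it calls PickUp only if the character's grabbed component belongs to this actor, gated by a DoOnce that resets when interaction stops.
; PickUp itself is left empty.
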(event OnComponentBeginOverlap(Box)
  (params (OverlappedComponent :type Primitive%20Component%20Object%20Reference) (OtherActor :type Actor%20Object%20Reference) (OtherComp :type Primitive%20Component%20Object%20Reference) (OtherBodyIndex :type Integer) (bFromSweep :type Boolean) (SweepResult :type Hit%20Result%20Structure%20%28by%20ref%29))
  ;[0.15 0.15 0.15 0.5] Verification & bind event
  (bind _asbp_garett (Utilities|Casting|CastToBP_Garett OtherActor))
  (bind _output_get (Variables|Default|SetCharacterRef _asbp_garett))
  (EventDispatchers|BindEventtoInteract _output_get (delegate Custom|CanPickUp)))

(event OnComponentEndOverlap(Box)
  (params (OverlappedComponent :type Primitive%20Component%20Object%20Reference) (OtherActor :type Actor%20Object%20Reference) (OtherComp :type Primitive%20Component%20Object%20Reference) (OtherBodyIndex :type Integer))
  ;[0.15 0.15 0.15 0.5] Unbind event
  (bind _asbp_garett (Utilities|Casting|CastToBP_Garett OtherActor))
  (EventDispatchers|UnbindEventfromInteract _asbp_garett (delegate Custom|CanPickUp)))

(event Custom|CanPickUp
  ;[0.15 0.15 0.15 0.5] Verify if can pick up
  (EventDispatchers|BindEventtoStoppedInteracting (Variables|Default|GetCharacterRef) (delegate Custom|ResetPickUp))
  (Utilities|FlowControl|DoOnce false
    (:Completed
      (if (== (Components|GetOwner (Variables|/Game/BluePrints/Character/Garett/BP_Garett.BP_Garett_C|GetGrabbedComponent (Variables|Default|GetCharacterRef))) self)
        (CallFunction|PickUp)))))

(event Custom|ResetPickUp
  ;[0.15 0.15 0.15 0.5] Verify if can pick up
  (Utilities|FlowControl|DoOnce false) ; enters at Reset
)

(event EventBeginPlay
  (bind _pickupobjectmesh (Variables|Default|GetPickUpObjectMesh))
  (Components|StaticMesh|SetStaticMesh _pickupobjectmesh (Variables|Default|GetPickUpMesh))
  (Physics|SetSimulatePhysics _pickupobjectmesh false))

(event Collision|EventActorBeginOverlap
  (params (OtherActor :type Actor%20Object%20Reference)))

(event EventTick
  (params (DeltaSeconds :type Float%20%28single-precision%29)))

(fn ConstructionScript
  (Components|StaticMesh|SetStaticMesh (Variables|Default|GetPickUpObjectMesh) (Variables|Default|GetPickUpMesh)))

(fn PickUp)