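; Moss zone actor that silences BP_Garett's noise while he stands inside it.
; On BeginPlay it traces up to 600 units down, snaps to the impact point or destroys itself if nothing is hit.
; A MossGrowth timeline then widens the Sphere in X and Y.
; Sphere overlap deactivates Garett's PawnNoiseEmitter on entry and reactivates it on exit.
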(event OnComponentBeginOverlap(Sphere)
  (params (OverlappedComponent :type Primitive%20Component%20Object%20Reference) (OtherActor :type Actor%20Object%20Reference) (OtherComp :type Primitive%20Component%20Object%20Reference) (OtherBodyIndex :type Integer) (bFromSweep :type Boolean) (SweepResult :type Hit%20Result%20Structure%20%28by%20ref%29))
  (bind _asbp_garett (Utilities|Casting|CastToBP_Garett OtherActor))
  (Components|Activation|Deactivate (Variables|/Game/BluePrints/Character/Garett/BP_Garett.BP_Garett_C|GetPawnNoiseEmitter _asbp_garett)))

(event OnComponentEndOverlap(Sphere)
  (params (OverlappedComponent :type Primitive%20Component%20Object%20Reference) (OtherActor :type Actor%20Object%20Reference) (OtherComp :type Primitive%20Component%20Object%20Reference) (OtherBodyIndex :type Integer))
  (bind _asbp_garett (Utilities|Casting|CastToBP_Garett OtherActor))
  (Components|Activation|Activate (Variables|/Game/BluePrints/Character/Garett/BP_Garett.BP_Garett_C|GetPawnNoiseEmitter _asbp_garett) false))

(event Custom|GrowMoss
  (bind _sphere (Variables|Default|GetSphere))
  (bind _growth (Timeline|MossGrowth Play)
    (:Update
      (Transformation|SetRelativeScale3D _sphere (Math|Vector|MakeVector (* _growth 1e+01) (* _growth 1e+01) (.z (Variables|/Script/Engine.SceneComponent|GetRelativeScale3D _sphere)))))))

(event EventBeginPlay
  (bind _returnvalue (Transformation|GetActorLocation))
  (bind _defaultsceneroot (Variables|Default|GetDefaultSceneRoot))
  (bind (_x _y _z) (Math|Vector|BreakVector _returnvalue))
  (bind _outhit (Collision|LineTraceByChannel _returnvalue (Math|Vector|MakeVector _x _y (- _z 6e+02)) "TraceTypeQuery1" false 0 "Persistent"))
  (if (.bBlockingHit (Collision|BreakHitResult _outhit))
    (Transformation|SetWorldTransform _defaultsceneroot (Math|Transform|MakeTransform (.ImpactPoint (Collision|BreakHitResult _outhit)) "0, 0, 0" (Transformation|GetWorldScale _defaultsceneroot)) false false)
    (CallFunction|GrowMoss)
    (else
      (Actor|DestroyActor))))

(event Collision|EventActorBeginOverlap
  (params (OtherActor :type Actor%20Object%20Reference)))

(event EventTick
  (params (DeltaSeconds :type Float%20%28single-precision%29)))

(fn ConstructionScript)