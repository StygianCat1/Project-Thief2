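; Water arrow variant of a parent arrow Blueprint that puts out torches.
; Its ExtiguishTorch override runs the parent logic, then calls CallExtinguishLights on the given torch.
; When its Box component registers a hit, it destroys the Sphere component if still valid.
; The construction script only calls the parent, and BeginPlay, Tick and overlap events are disabled stubs.
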(event OnComponentHit(Box)
  (params (HitComponent :type Primitive%20Component%20Object%20Reference) (OtherActor :type Actor%20Object%20Reference) (OtherComp :type Primitive%20Component%20Object%20Reference) (NormalImpulse :type Vector :default "0, 0, 0") (Hit :type Hit%20Result%20Structure%20%28by%20ref%29))
  (bind _sphere (Variables|Default|GetSphere)
    (:then
      (Components|DestroyComponent _sphere))
    (:else)))

(event EventBeginPlay
  (|CallParentFunction) ; This node is disabled and will not be called.\nDrag off pins to build functionality.
)

(event Collision|EventActorBeginOverlap
  (params (OtherActor :type Actor%20Object%20Reference))
  (|CallParentFunction OtherActor) ; This node is disabled and will not be called.\nDrag off pins to build functionality.
)

(event EventTick
  (params (DeltaSeconds :type Float%20%28single-precision%29))
  (|CallParentFunction DeltaSeconds) ; This node is disabled and will not be called.\nDrag off pins to build functionality.
)

(fn ConstructionScript
  (|CallParentFunction))

(fn ExtiguishTorch
  (params (TorchRef :type BP%20Torch%20Object%20Reference))
  (|CallParentFunction TorchRef)
  (Default|CallExtinguishLights TorchRef))