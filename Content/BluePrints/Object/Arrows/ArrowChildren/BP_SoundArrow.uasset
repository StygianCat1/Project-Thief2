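; BP_SoundArrow is an arrow variant that creates a noise source where it strikes.
; On the first hit of its Box component, a DoOnce gate spawns a BP_ArrowNoiseEmitter at the Box's world transform, ignoring spawn collisions.
; The construction script only calls the parent, and the BeginPlay, overlap and Tick stubs are disabled.
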(event OnComponentHit(Box)
  (params (HitComponent :type Primitive%20Component%20Object%20Reference) (OtherActor :type Actor%20Object%20Reference) (OtherComp :type Primitive%20Component%20Object%20Reference) (NormalImpulse :type Vector :default "0, 0, 0") (Hit :type Hit%20Result%20Structure%20%28by%20ref%29))
  (Utilities|FlowControl|DoOnce false
    (:Completed
      (Game|SpawnActorfromClass "/Game/BluePrints/Object/Arrows/ArrowsCreation/BP_ArrowNoiseEmitter.BP_ArrowNoiseEmitter_C" (Transformation|GetWorldTransform (Variables|Default|GetBox)) "AlwaysSpawn" "MultiplyWithRoot" 0 0))))

(event EventBeginPlay
  (|CallParentFunction) ; This node is disabled and will not be called.\nDrag off pins to build functionality.
)

(event Collision|EventActorBeginOverlap
  (params (OtherActor :type Actor%20Object%20Reference))
  (|CallParentFunction OtherActor) ; This node is disabled and will not be called.\nDrag off pins to build functionality.
)

(event EventTick
  (params (DeltaSeconds :type Float%20%28single-precision%29))
  (|CallParentFunction DeltaSeconds) ; This node is disabled and will not be called.\nDrag off pins to build functionality.
)

(fn ConstructionScript
  (|CallParentFunction))