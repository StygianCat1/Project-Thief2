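; BP_ScoutingOrb is a possessable scouting orb that gives the player a look-around camera where it hits.
; When its sphere registers a hit, player controller 0 switches view to the orb and possesses it.
; Mouse and look inputs share a Look function that rotates the camera in world space with inverted pitch input.
; The quit-possession input returns view and control to the BP_Garett character cached on BeginPlay.
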(event OnComponentHit(Sphere)
  (params (HitComponent :type Primitive%20Component%20Object%20Reference) (OtherActor :type Actor%20Object%20Reference) (OtherComp :type Primitive%20Component%20Object%20Reference) (NormalImpulse :type Vector :default "0, 0, 0") (Hit :type Hit%20Result%20Structure%20%28by%20ref%29))
  (bind _returnvalue (Game|GetPlayerController 0))
  (bind _self self)
  (Game|Player|SetViewTargetwithBlend _returnvalue _self 0.0 "VTBlend_Linear" 0.0 false)
  (Pawn|Possess _returnvalue _self))

(event Input|EnhancedActionEvents|EnhancedInputActionIA_MouseLook
  (params (ActionValue :type Vector%202D%20Structure) (ElapsedSeconds :type Float%20%28double-precision%29) (TriggeredSeconds :type Float%20%28double-precision%29) (InputAction :type Input%20Action%20Object%20Reference :default "/Game/BluePrints/Input/Actions/IA_MouseLook.IA_MouseLook"))
  (CallFunction|Look (.x ActionValue) (.y ActionValue)))

(event Input|EnhancedActionEvents|EnhancedInputActionIA_QuitPossesion
  (params (ActionValue :type Boolean) (ElapsedSeconds :type Float%20%28double-precision%29) (TriggeredSeconds :type Float%20%28double-precision%29) (InputAction :type Input%20Action%20Object%20Reference :default "/Game/BluePrints/Input/Actions/IA_QuitPossesion.IA_QuitPossesion"))
  (bind _returnvalue (Game|GetPlayerController 0))
  (bind _characterref (Variables|Default|GetCharacterRef))
  (Game|Player|SetViewTargetwithBlend _returnvalue _characterref 0.0 "VTBlend_Linear" 0.0 false)
  (Pawn|Possess _returnvalue _characterref))

(event Input|EnhancedActionEvents|EnhancedInputActionIA_Look
  (params (ActionValue :type Vector%202D%20Structure) (ElapsedSeconds :type Float%20%28double-precision%29) (TriggeredSeconds :type Float%20%28double-precision%29) (InputAction :type Input%20Action%20Object%20Reference :default "/Game/BluePrints/Input/Actions/IA_Look.IA_Look"))
  (CallFunction|Look (.x ActionValue) (.y ActionValue)))

(event EventBeginPlay
  (|CallParentFunction)
  (bind _returnvalue (Actor|GetActorOfClass "/Game/BluePrints/Character/Garett/BP_Garett.BP_Garett_C"))
  (Variables|Default|SetCharacterRef _returnvalue))

(event Collision|EventActorBeginOverlap
  (params (OtherActor :type Actor%20Object%20Reference)))

(event EventTick
  (params (DeltaSeconds :type Float%20%28single-precision%29)))

(fn ConstructionScript
  (|CallParentFunction))

(fn Look
  (params (Yaw :type Float%20%28single-precision%29) (Pitch :type Float%20%28double-precision%29))
  (bind _camera (Variables|Default|GetCamera))
  (bind _returnvalue (Transformation|GetWorldRotation _camera))
  (Transformation|SetWorldRotation (Variables|Default|GetCamera) (Math|Rotator|MakeRotator (.roll _returnvalue) (+ (.pitch _returnvalue) (* Pitch -1.0)) (+ (.yaw _returnvalue) Yaw)) false false))