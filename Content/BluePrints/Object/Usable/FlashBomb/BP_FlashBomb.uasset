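; BP_FlashBomb is a usable flash bomb that detonates 1.5 seconds after spawning, flashing the player and stunning nearby AI.
; StunCharacter adds the WBP_Flashbang widget to the viewport without any range check, then destroys the actor after a short delay.
; StunIA runs during that delay, looping over all BP_AIBase actors and calling CallStunned on those within a fixed radius of the bomb.
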(event Custom|StunIA
  ;[0.15 0.15 0.15 0.5] Flash & stun IA_enemy in proximity
  (bind _outactors (Actor|GetAllActorsOfClass "/Game/BluePrints/Character/IAs/BP_AIBase.BP_AIBase_C"))
  (for _array_element _outactors
    (if (<= (Math|Vector|Distance(Vector) (Transformation|GetActorLocation _array_element) (Transformation|GetActorLocation)) 2e+03)
      (Default|CallStunned _array_element))))

(event Custom|StunCharacter
  ;[0.15 0.15 0.15 0.5] Flash character
  (bind _returnvalue (UserInterface|CreateWidget "/Game/UI/InGame/WBP_Flashbang.WBP_Flashbang_C"))
  (UserInterface|Viewport|AddtoViewport _returnvalue 0)
  (Utilities|FlowControl|Delay 0.2)
  (Actor|DestroyActor))

(event EventBeginPlay
  ;[0.15 0.15 0.15 0.5] Set up & launch flash
  (|CallParentFunction)
  (Utilities|FlowControl|Delay 1.5)
  (CallFunction|StunCharacter)
  (CallFunction|StunIA))

(fn ConstructionScript
  (|CallParentFunction))